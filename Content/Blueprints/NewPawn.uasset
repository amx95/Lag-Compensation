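; Test pawn for server-side hit verification against a player's location history, in the style of lag compensation.
; Left click traces from the camera, marks BP_PlayerCharacter hits with a debug sphere, and sends location, time and actor for checking.
; The target's CheckHit result is printed, and the approved historical location gets a second sphere.
; The autonomous proxy adds a crosshair and starts a looping timer, alongside events that manually replicate pawn location and control rotation.
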(event `GetServerAproove`
  (params (AprooveLocation :type "Vector Structure"))
  (`KismetSystemLibrary.DrawDebugSphere` AprooveLocation 15.0 12 (struct :`R` 1.0 :`B` 0.261998 :`A` 1.0) 10.0 1.0))

(event `CustomReplicateMovement`
  (params (Rotation :type "Rotator Structure") (Location :type "Vector Structure"))
  (`self.K2_SetActorLocation` Location)
  (`self.K2_SetActorRotation` Rotation))

(event `self.ReceiveBeginPlay`
  (if (`|EnumEquality` (`self.GetLocalRole`) "ROLE_AutonomousProxy")
    (`KismetSystemLibrary.K2_SetTimerDelegate` (`|CreateDelegate` :!event `SendMovementToServer`) 0.5 true)
    (bind _returnvalue (`|CreateWidget` "/Game/UI_CrossHair.UI_CrossHair_C"))
    (`UserWidget.AddToPlayerScreen` _returnvalue 0)))

(event `Server_CheckHit`
  (params (HitLocation :type "Vector Structure") (HitTime :type "Float (double-precision)") (HitActor :type "/Game/BP_PlayerCharacter Object Reference"))
  (bind (_success _distance _betweentime _locationinhistory _timeinhistory) (`MyCharacter.CheckHit` HitActor HitLocation HitTime))
  (if _success
    (`KismetSystemLibrary.PrintString` (`KismetTextLibrary.Conv_TextToString` (`|FormatText` "Server Location in History {SLIH} \nServer LocationTime in History {SLTINH} \nActualSimulatedClientHitLocatin {ASCH} \nDistanceBetweenVectors {DBV} \nBetweenTime {Time}" (`KismetTextLibrary.Conv_VectorToText` _locationinhistory) _timeinhistory (`KismetStringLibrary.Conv_VectorToString` HitLocation) _distance _betweentime)) true true (struct :`R` 1.0 :`B` 0.720657 :`A` 1.0) 10.0)
    (`self.GetServerAproove` _locationinhistory)))

(event `SendMovementToServer`
  (`self.CustomReplicateMovement` (`self.GetControlRotation`) (`self.K2_GetActorLocation`)))

(event `Key|LeftMouseButton`
  (params (Key :type "Key Structure"))
  (bind _camera (`self.Camera`))
  (bind _returnvalue (`SceneComponent.K2_GetComponentLocation` _camera))
  (:`Pressed`
    (bind (_outhit _returnvalue_2) (`KismetSystemLibrary.LineTraceSingle` :`Start` (+ _returnvalue (0.0 0.0 -1.0)) :`End` (+ _returnvalue (* (`SceneComponent.GetForwardVector` _camera) 1000.0)) :`TraceChannel` "TraceTypeQuery2" :`DrawDebugType` "ForDuration" :`DrawTime` 1.0))
    (if _returnvalue_2
      (bind (_bblockinghit _binitialoverlap _time _distance _location _impactpoint _normal _impactnormal _physmat _hitactor) (`GameplayStatics.BreakHitResult` _outhit))
      (bind _asbp_player_character (cast `/Game/BP_PlayerCharacter` _hitactor))
      (`KismetSystemLibrary.DrawDebugSphere` _location 15.0 8 (struct :`R` 0.311043 :`G` 1.0 :`A` 1.0) 10.0 1.0)
      (`self.Server_CheckHit` _location (`KismetSystemLibrary.GetGameTimeInSeconds`) _asbp_player_character))))

(fn `UserConstructionScript`)